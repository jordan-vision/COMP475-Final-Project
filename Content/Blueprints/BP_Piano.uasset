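; BP_Piano is a five-key piano actor that plays C, D, E, G and A notes when its key components register hits.
; On BeginPlay it loads a piano SoundCue into a child BP_Speaker's audio component, allowing overlapping instances.
; Each hit runs its key's Play function, which swaps the cue's "Note" wave parameter, though PlayD uses the E wave.
; A DoOnce with a short delayed reset debounces each key.
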(event EventBeginPlay
  (bind _asbp_speaker (Utilities|Casting|CastToBP_Speaker (Variables|/Script/Engine.ChildActorComponent|GetChildActor (Variables|Default|GetBP_Speaker))))
  (bind _output_get (Variables|Default|SetSpeakerAudioComponent (Variables|/Game/Blueprints/BP_Speaker.BP_Speaker_C|GetAudio _asbp_speaker)))
  (bind _output_get_2 (Variables|Components|SetSoundCue "/Game/Audio/SC_Piano.SC_Piano"))
  (Audio|Components|Audio|SetSound _output_get _output_get_2)
  (Variables|/Script/Engine.AudioComponent|SetbCanPlayMultipleInstances _output_get true))

(event Collision|EventActorBeginOverlap
  (params (OtherActor :type Actor%20Object%20Reference)))

(event EventTick
  (params (DeltaSeconds :type Float%20%28single-precision%29)))

(event Collision|EventHit
  (params (MyComp :type Primitive%20Component%20Object%20Reference) (Other :type Actor%20Object%20Reference) (OtherComp :type Primitive%20Component%20Object%20Reference) (bSelfMoved :type Boolean) (HitLocation :type Vector :default "0, 0, 0") (HitNormal :type Vector :default "0, 0, 0") (NormalImpulse :type Vector :default "0, 0, 0") (Hit :type Hit%20Result%20Structure%20%28by%20ref%29))
  (if (== MyComp (Variables|Default|GetC))
    (Utilities|FlowControl|DoOnce false :!label _label
      (:Completed
        (CallFunction|PlayC)
        (Utilities|FlowControl|Delay 0.1)
        (goto _label Reset)))
    (elif (== MyComp (Variables|Default|GetD))
      (Utilities|FlowControl|DoOnce false :!label _label_2
        (:Completed
          (CallFunction|PlayD)
          (Utilities|FlowControl|Delay 0.1)
          (goto _label_2 Reset)))
      (elif (== MyComp (Variables|Default|GetE))
        (Utilities|FlowControl|DoOnce false :!label _label_3
          (:Completed
            (CallFunction|PlayE)
            (Utilities|FlowControl|Delay 0.1)
            (goto _label_3 Reset)))
        (elif (== MyComp (Variables|Default|GetG))
          (Utilities|FlowControl|DoOnce false :!label _label_4
            (:Completed
              (CallFunction|PlayG)
              (Utilities|FlowControl|Delay 0.1)
              (goto _label_4 Reset)))
          (elif (== MyComp (Variables|Default|GetA))
            (Utilities|FlowControl|DoOnce false :!label _label_5
              (:Completed
                (CallFunction|PlayA)
                (Utilities|FlowControl|Delay 0.1)
                (goto _label_5 Reset)))))))))

(fn ConstructionScript)

(fn PlayC
  (bind _speakeraudiocomponent (Variables|Default|GetSpeakerAudioComponent))
  (Class|AudioComponent|SetWaveParameter _speakeraudiocomponent "Note" "/Game/Audio/PianoC.PianoC")
  (Audio|Components|Audio|Play _speakeraudiocomponent 0.0))

(fn PlayD
  (bind _speakeraudiocomponent (Variables|Default|GetSpeakerAudioComponent))
  (Class|AudioComponent|SetWaveParameter _speakeraudiocomponent "Note" "/Game/Audio/PianoE.PianoE")
  (Audio|Components|Audio|Play _speakeraudiocomponent 0.0))

(fn PlayE
  (bind _speakeraudiocomponent (Variables|Default|GetSpeakerAudioComponent))
  (Class|AudioComponent|SetWaveParameter _speakeraudiocomponent "Note" "/Game/Audio/PianoE.PianoE")
  (Audio|Components|Audio|Play _speakeraudiocomponent 0.0))

(fn PlayG
  (bind _speakeraudiocomponent (Variables|Default|GetSpeakerAudioComponent))
  (Class|AudioComponent|SetWaveParameter _speakeraudiocomponent "Note" "/Game/Audio/PianoG.PianoG")
  (Audio|Components|Audio|Play _speakeraudiocomponent 0.0))

(fn PlayA
  (bind _speakeraudiocomponent (Variables|Default|GetSpeakerAudioComponent))
  (Class|AudioComponent|SetWaveParameter _speakeraudiocomponent "Note" "/Game/Audio/PianoA.PianoA")
  (Audio|Components|Audio|Play _speakeraudiocomponent 0.0))