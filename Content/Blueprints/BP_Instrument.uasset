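; BP_Instrument is an instrument actor with start and stop buttons, linked to a BP_Speaker child actor.
; On BeginPlay it caches the speaker's audio component and stores the vibraphone sound cue.
; Hits on either button component only print a start or stop message, with no playback wired up.
; A bool parameter call on the sound cue is left unconnected.
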(event EventBeginPlay
  (bind _asbp_speaker (Utilities|Casting|CastToBP_Speaker (Variables|/Script/Engine.ChildActorComponent|GetChildActor (Variables|Default|GetBP_Speaker))))
  (Variables|Default|SetSpeakerAudioComponent (Variables|/Game/Blueprints/BP_Speaker.BP_Speaker_C|GetAudio _asbp_speaker))
  (Variables|Default|SetSoundCue "/Game/Sounds/SC_Vibraphone.SC_Vibraphone"))

(event Collision|EventActorBeginOverlap
  (params (OtherActor :type Actor%20Object%20Reference)))

(event EventTick
  (params (DeltaSeconds :type Float%20%28single-precision%29)))

(event Collision|EventHit
  (params (MyComp :type Primitive%20Component%20Object%20Reference) (Other :type Actor%20Object%20Reference) (OtherComp :type Primitive%20Component%20Object%20Reference) (bSelfMoved :type Boolean) (HitLocation :type Vector :default "0, 0, 0") (HitNormal :type Vector :default "0, 0, 0") (NormalImpulse :type Vector :default "0, 0, 0") (Hit :type Hit%20Result%20Structure%20%28by%20ref%29))
  (if (== MyComp (Variables|Default|GetStartButton))
    (Development|PrintString "Start Music")
    (elif (== MyComp (Variables|Default|GetStopButton))
      (Development|PrintString "Stop Music"))))

(fn ConstructionScript)